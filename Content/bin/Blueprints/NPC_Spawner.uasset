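; Spawner actor that populates its surroundings with NPC_Peaton pedestrians while the player is nearby.
; After a random startup delay it enables Tick, which triggers spawning whenever the player is within SpawnerRange.
; A DoOnce-guarded delayed loop spawns NPCs at random reachable nearby points, gives them controllers and refills to RequiredNPCCount.
; Every tick also culls tracked NPCs beyond NPCRange from the player, freeing slots for respawning.
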(event Custom|SpawnNPCS
  (Utilities|FlowControl|DoOnce false :!label _label
    (:Completed
      (if (> (Variables|Default|GetRequiredNPCCount) (Variables|Default|GetSpawnedNPCCount)) :!label _label_2
        (bind _returnvalue (Game|SpawnActorfromClass "/Game/bin/Blueprints/NPC_Peaton.NPC_Peaton_C" (Math|Transform|MakeTransform (.RandomLocation (AI|Navigation|GetRandomReachablePointinRadius (Transformation|GetActorLocation) 5e+02 0 0)) (Math|Rotator|MakeRotator 0.0 0.0 (Math|Random|RandomFloatinRange 0.0 3.6e+02)) "1,1,1") "AdjustIfPossibleButAlwaysSpawn" 0 "/Game/Modelos/NPC/aj.aj" "/Game/Modelos/NPC/aj_Skeleton_AnimBlueprint.aj_Skeleton_AnimBlueprint_C" 0))
        (Utilities|IsValid _returnvalue
          (:Is%20Valid
            (Utilities|Array|Add (Variables|Default|GetSpawnedNPCS) _returnvalue)
            (Math|Integer|IncrementInt (Variables|Default|GetSpawnedNPCCount)
              (:%20%20
                (Utilities|FlowControl|Delay 0.2)
                (Pawn|SpawnDefaultController _returnvalue)
                (goto _label_2)))))
        (else
          (goto _label Reset))))))

(event EventBeginPlay
  (Utilities|FlowControl|Delay (Math|Random|RandomFloatinRange 0.5 2.0))
  (Actor|Tick|SetActorTickEnabled true))

(event EventTick
  (params (DeltaSeconds :type Float%20%28single-precision%29))
  (if (< (Utilities|GetDistancetoPlayer self) (Variables|Default|GetSpawner_Range))
    (CallFunction|SpawnNPCS))
  (CallFunction|CheckNPCLocations))

(fn ConstructionScript)

(fn CheckNPCLocations
  (bind _spawnednpcs (Variables|Default|GetSpawnedNPCS))
  (for _array_element _spawnednpcs
    (Utilities|IsValid _array_element
      (:Is%20Valid
        (if (> (Utilities|GetDistancetoPlayer _array_element) (Variables|Default|GetNPCRange))
          (Utilities|Array|RemoveItem _spawnednpcs _array_element)
          (Utilities|IsValid _array_element
            (:Is%20Valid
              (Actor|DestroyActor _array_element)
              (Math|Integer|DecrementInt (Variables|Default|GetSpawnedNPCCount)))))))))