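; Jugador is the shared character Blueprint for every playable character, configured by Tipo and acting as player or following ally via Aliado.
; Input handles sprint, punch, character switching through a level event, character quirks and inventory.
; Tick runs controllers for ragdoll and death (level restarts when no allies survive), plus Danny-only bladder and line-trace look-at with tooltip and outline.
; That trace feeds interaction keys, while functions add, use and drop items in an inventory map.
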(event Custom|Follow%20Player
  (bind _self self)
  (bind _player_ref (Variables|Default|GetPlayer%20REF))
  ;[1 1 1] Seguir al Jugador
  (if (>= (Transformation|GetDistanceTo _player_ref) 4e+02)
    ;;[1 1 1] Si aun hay distancia va hacia el
    (AI|AIMoveTo _self "0, 0, 0" _player_ref 5.0 false
      (:then
        _))
    (else
      ;;[1 1 1] Si distancia es inferior se para
      (AI|AIMoveTo _self "0, 0, 0" _self 5.0 false
        (:then
          _))))
  ;;[1 1 1] Cada medio segundo se vuelve a lanzar
  (Utilities|FlowControl|Delay 0.5)
  (CallFunction|FollowPlayer))

(event Custom|RagdollCapsuleController
  ;[1 1 1] CONTROLLERS
  ;;[1 1 1] Mantener capsula cuando entramos en Ragdoll
  (if (Variables|Estado|GetRagdoll)
    (Transformation|SetWorldLocation (Variables|Default|GetCapsuleComponent) (+ (Transformation|GetSocketLocation (Variables|Character|GetMesh) "Hips") "0, 0,95.000000") false false)))

(event Custom|DeathController
  (bind _returnvalue (Game|GetPlayerController 0))
  ;[1 1 1] CONTROLLERS
  ;;[1 1 1] Muerte del Jugador
  ;;;[1 1 1] Para que no se repita varias veces, comprobamos que el jugador sigue vivo
  (if (and (not (Variables|Estado|GetMuerto)) (<= (Variables|Atributos|GetVida) 0.0))
    (Variables|Estado|SetMuerto true)
    ;;;[1 1 1] Activar Ragdoll
    (Class|SkeletalMeshComponent|SetAllBodiesBelowSimulatePhysics (Variables|Character|GetMesh) (Utilities|Name|MakeLiteralName "hips") true true)
    (Variables|Estado|SetRagdoll true)
    ;;;[1 1 1] Si es el Jugador
    (if (not (Variables|Estado|GetAliado))
      ;;;[1 1 1] Reset variable antes de comprobar
      (Variables|Default|SetHasAllies? false)
      ;;;[1 1 1] Comprobar si queda algun aliado con vida
      (bind _array_element (Utilities|Array|ForEachLoopwithBreak (Variables|Default|GetAliados) :!label _label)
        (:LoopBody
          (if (not (Variables|Jugador_C|GetMuerto _array_element))
            (Variables|Default|SetHasAllies? true)
            (goto _label Break)))
        (:Completed
          ;;;[1 1 1] WASTED solo cuando no le quedan aliados
          (if (not (Variables|Default|GetHasAllies?))
            ;;;[1 1 1] Deshabilitar inputs
            (Input|SetInputModeUIOnly _returnvalue 0 "DoNotLock")
            ;;;[1 1 1] Pantalla blanco y negro
            (Utilities|Struct|SetmembersinPostProcessSettings (Variables|/Script/Engine.CameraComponent|GetPostProcessSettings (Variables|Default|GetFollowCamera)) (Variables|Default|GetSaturation))
            ;;;[1 1 1] Quitar HUD
            (Viewport|RemoveAllWidgets)
            (Audio|PlaySound2D "/Game/OST/efectos/muerte.muerte" 1.0 1.0 0.0 0 0)
            (Utilities|FlowControl|Delay 3.0)
            ;;;[1 1 1] Wasted
            (bind _returnvalue_2 (UserInterface|CreateWidget "/Game/UI/Muerte.Muerte_C" _returnvalue))
            (UserInterface|Viewport|AddtoViewport _returnvalue_2 0)
            (Utilities|FlowControl|Delay 5.25)
            ;;;[1 1 1] Reiniciar nivel
            (bind _returnvalue_3 (Game|GetCurrentLevelName true))
            (Game|OpenLevel(byName) (Utilities|String|StringToName _returnvalue_3))
            (Input|SetInputModeGameOnly _returnvalue)))))))

(event Custom|PlayerLookingController
  (bind _returnvalue (Transformation|GetActorLocation))
  (bind _interactuarwidget (Variables|UI|GetInteractuarWidget))
  ;[1 1 1] CONTROLLERS
  ;;[1 1 1] Comprueba si el Jugador esta mirando un objeto
  ;;;[1 1 1] Sensor desde nuestro actor, con la direccion a la que apunta la camara, 180 cm adelante
  (bind (_outhit _returnvalue_2) (Collision|LineTraceByChannel _returnvalue (+ _returnvalue (* (Math|Vector|GetForwardVector (Variables|Default|GetFollowCamera)) 1.8e+02)) "TraceTypeQuery1" false 0 "None"))
  (if (and _returnvalue_2 (Utilities|ClassIsChildOf (Utilities|GetClass (.HitActor (Collision|BreakHitResult _outhit))) "/Game/bin/Blueprints/InteractiveObject.InteractiveObject_C"))
    ;;;[1 1 1] Le pasa el mensaje de interaccion correspondiente a la UI
    (bind _asinteractive_object (Utilities|Casting|CastToInteractiveObject (.HitActor (Collision|BreakHitResult _outhit))))
    (Default|ObtenerMensaje _interactuarwidget (Variables|/Game/bin/Blueprints/InteractiveObject.InteractiveObject_C|GetMensajeInteraccion _asinteractive_object))
    ;;[1 1 1] Obtenemos la info de tabla para agregarlo al Inventario, usarlo o equiparlo
    (bind _atributos (Default|ObtenerInfoItem _interactuarwidget (Variables|/Game/bin/Blueprints/InteractiveObject.InteractiveObject_C|GetItem _asinteractive_object)))
    (Variables|/Game/bin/Blueprints/InteractiveObject.InteractiveObject_C|SetAtributos _asinteractive_object _atributos)
    ;;[1 1 1] Saca el Tooltip
    (Widget|SetVisibility _interactuarwidget "Visible")
    ;;[1 1 1] Mostrar delineado cuando NO es puerta y obtener info del item
    (Utilities|Casting|CastToPuertaBP (.HitActor (Collision|BreakHitResult _outhit))
      (:CastFailed
        (bind _output_get (Variables|Default|SetItemSeleccionado (.HitComponent (Collision|BreakHitResult _outhit))))
        (Rendering|SetRenderCustomDepth _output_get true)))
    (else
      ;;[1 1 1] Quita Tooltip
      (Widget|SetVisibility _interactuarwidget "Hidden")
      (if (Utilities|IsValid (Variables|Default|GetItemSeleccionado))
        ;;[1 1 1] Quitar delineado y reset item
        (Rendering|SetRenderCustomDepth (Variables|Default|GetItemSeleccionado) false)
        (Variables|Default|SetItemSeleccionado 0)))))

(event Custom|RestarVejiga
  (Variables|Atributos|SetVejiga (+ (Variables|Atributos|GetVejiga) 1.0)))

(event Custom|SetAliados
  (params (Player%20REF :type Jugador%20Object%20Reference))
  ;[1 1 1] Checkea y setea conducta de Aliados actuales
  ;;[1 1 1] Ref. al Jugador para Aliados
  (Variables|Default|SetPlayer%20REF Player%20REF)
  ;;[1 1 1] TRUE es Solo para Aliados, FALSE solo para el Jugador
  (if (Variables|Estado|GetAliado)
    ;;[1 1 1] Trigger para Seguir al Jugador
    (CallFunction|FollowPlayer)
    ;;[1 1 1] Quitar mensajes y delineados residuales por si acabamos de cambiar de Jugador
    (Widget|SetVisibility (Variables|UI|GetInventarioWidget) "Hidden")
    (Widget|SetVisibility (Variables|UI|GetInteractuarWidget) "Hidden")
    (if (Utilities|IsValid (Variables|Default|GetItemSeleccionado))
      (Rendering|SetRenderCustomDepth (Variables|Default|GetItemSeleccionado) false)
      (Variables|Default|SetItemSeleccionado 0))
    (else
      ;;[1 1 1] Check de Aliados en el Nivel - Esta aqui y no en el LevelBP porque se hace tambien al principio del juego, y para niveles en los que no puedas cambiar
      (bind _outactors (Actor|GetAllActorsOfClass "Jugador_C"))
      (bind _output_get (Variables|Default|SetAliados _outactors))
      ;;;[1 1 1] Eliminamos del array al propio jugador
      (Utilities|Array|RemoveIndex _output_get (Utilities|Array|FindItem _output_get (Variables|Default|GetPlayer%20REF))))))

(event Custom|VejigaController
  (bind _mesh (Variables|Character|GetMesh))
  (bind _charactermovement (Variables|Character|GetCharacterMovement))
  ;[1 1 1] CONTROLLERS
  ;;[1 1 1] Check de la Vejiga de Danny
  (if (>= (Variables|Atributos|GetVejiga) 1e+02)
    ;;;[1 1 1] Vaciamos vejiga lo primero para evitar que se lance el evento otra vez
    (Variables|Atributos|SetVejiga 0.0)
    ;;;[1 1 1] Deshabilita movimiento, pero no camara
    (Pawn|Components|CharacterMovement|DisableMovement _charactermovement)
    ;;;[1 1 1] Que se mea
    (Components|Animation|PlayAnimation _mesh "/Game/Modelos/Danny/Animaciones/Injured_Hurting_Idle.Injured_Hurting_Idle" false)
    (Utilities|FlowControl|Delay 4.0)
    ;;;[1 1 1] Se meo
    (AddComponent|AddParticleSystemComponent false)
    (bind _returnvalue (AddComponent|AddParticleSystemComponent false))
    (Utilities|FlowControl|Delay 6.0)
    ;;;[1 1 1] Vuelta a la normalidad
    (Components|Activation|ToggleActive _returnvalue)
    (Components|Animation|SetAnimationMode _mesh "AnimationBlueprint")
    (Pawn|Components|CharacterMovement|SetMovementMode _charactermovement "MOVE_Walking" 0)))

(event EventTick
  (params (DeltaSeconds :type Float%20%28single-precision%29))
  ;[1 1 1] Controllers que checkean cada medio segundo
  (CallFunction|RagdollCapsuleController)
  (CallFunction|DeathController)
  (switch Utilities|FlowControl|Switch|SwitchonJugadores (Variables|Atributos|GetTipo)
    (:NewEnumerator0
      ;;[1 1 1] Controllers custom
      (CallFunction|VejigaController)
      ;;[1 1 1] Los allies NO deben ejecutar estos controllers
      (if (not (Variables|Estado|GetAliado))
        (CallFunction|PlayerLookingController)))))

(event Game|Damage|EventRadialDamage
  (params (DamageReceived :type Float%20%28single-precision%29) (DamageType :type Damage%20Type%20Object%20Reference) (Origin :type Vector :default "0, 0, 0") (HitInfo :type Hit%20Result%20Structure%20%28by%20ref%29) (InstigatedBy :type Controller%20Object%20Reference) (DamageCauser :type Actor%20Object%20Reference))
  ;[1 1 1] Restar vida segun Enemigo
  (bind _returnvalue (Actor|GetActorOfClass (Utilities|GetClass DamageCauser)))
  (switch string (Utilities|String|ToString(Object) _returnvalue)
    (:Default
      (Variables|Default|SetDamage 1e+01))
    (:Hector
      (Variables|Default|SetDamage 1e+01)))
  (Variables|Atributos|SetVida (- (Variables|Atributos|GetVida) (Variables|Default|GetDamage))))

(event EventBeginPlay
  (bind _returnvalue (Game|GetPlayerController 0))
  (Utilities|Time|SetTimerbyEvent (delegate Custom|RestarVejiga) 5.0 true)
  ;[1 1 1] Metemos el Tooltip de Interactuar para mostrarlo cuando proceda
  (bind _returnvalue_2 (UserInterface|CreateWidget "/Game/UI/Interactuar.Interactuar_C" _returnvalue))
  (bind _output_get (Variables|UI|SetInteractuarWidget _returnvalue_2))
  (UserInterface|Viewport|AddtoViewport _output_get 0)
  ;[1 1 1] Tambien el Inventario
  (bind _returnvalue_3 (UserInterface|CreateWidget "/Game/UI/Inventario.Inventario_C" _returnvalue))
  (bind _output_get_2 (Variables|UI|SetInventarioWidget _returnvalue_3))
  (UserInterface|Viewport|AddtoViewport _output_get_2 0)
  (bind _asjugador (Utilities|Casting|CastToJugador (Game|Player|GetPlayerPawn 0)))
  ;[1 1 1] Declaramos atributos segun PJ
  (switch Utilities|FlowControl|Switch|SwitchonJugadores (Variables|Atributos|GetTipo)
    (:NewEnumerator0
      (Variables|Atributos|SetAtributos (Utilities|Struct|MakeAtributos 1.2e+03 100 100 1.3e+02)))
    (:NewEnumerator1
      (Variables|Atributos|SetAtributos (Utilities|Struct|MakeAtributos 1.2e+03 100 100 1e+02)))
    (:NewEnumerator2
      (Variables|Atributos|SetAtributos (Utilities|Struct|MakeAtributos 1.2e+03 100 100 1e+02)))
    (:NewEnumerator3
      (Variables|Atributos|SetAtributos (Utilities|Struct|MakeAtributos 1e+02 100 100 1e+02)))
    (:NewEnumerator4
      (Variables|Atributos|SetAtributos (Utilities|Struct|MakeAtributos 1e+02 100 100 1e+02)))
    (:NewEnumerator5
      (Variables|Atributos|SetAtributos (Utilities|Struct|MakeAtributos 1.2e+03 100 100 1e+02))))
  ;[1 1 1] Seteamos
  (Variables|Atributos|SetVida (.vida (Variables|Atributos|GetAtributos)))
  (Variables|Atributos|SetAtaque (.ataque (Variables|Atributos|GetAtributos)))
  (Variables|Atributos|SetVelocidad (.velocidad (Variables|Atributos|GetAtributos)))
  (Variables|Atributos|SetDefensa (.defensa (Variables|Atributos|GetAtributos)))
  (CallFunction|SetAliados _asjugador))

(event Input|KeyboardEvents|LeftShift
  (params (Key :type Key%20Structure :default "None"))
  (bind _charactermovement (Variables|Character|GetCharacterMovement))
  (bind _aliados (Variables|Default|GetAliados))
  ;[1 1 1] Esprintar
  (:Pressed
    (bind _output_get (Variables|/Script/Engine.CharacterMovementComponent|SetMaxWalkSpeed _charactermovement (Variables|Atributos|GetVelocidad)))
    ;[1 1 1] Igualar velocidad Aliados
    (for _array_element _aliados
      (Variables|/Script/Engine.CharacterMovementComponent|SetMaxWalkSpeed (Variables|/Script/Engine.Character|GetCharacterMovement _array_element) (- _output_get 1e+02))))
  (:Released
    (bind _output_get_2 (Variables|/Script/Engine.CharacterMovementComponent|SetMaxWalkSpeed _charactermovement 6e+02))
    (for _array_element_2 _aliados
      (Variables|/Script/Engine.CharacterMovementComponent|SetMaxWalkSpeed (Variables|/Script/Engine.Character|GetCharacterMovement _array_element) (- _output_get_2 1e+02)))))

(event Input|KeyboardEvents|V
  (params (Key :type Key%20Structure :default "None"))
  (:Pressed
    (switch Utilities|FlowControl|Switch|SwitchonJugadores (Variables|Atributos|GetTipo)
      (:NewEnumerator0
        ;[1 1 1] Danny - Tirarse pedo
        (Audio|SpawnSoundatLocation "/Game/OST/efectos/pedo1.pedo1" (Transformation|GetActorLocation) "0, 0, 0" 1.0 1.0 0.0 0 0))
      (:NewEnumerator2
        ;[1 1 1] Kathe - Fumar
        (Components|Animation|PlayAnimation (Variables|Character|GetMesh) "/Game/Modelos/Kathe/Animaciones/Smoking.Smoking" false)
        (Utilities|FlowControl|Delay 6.0)
        (bind _returnvalue (AddComponent|AddParticleSystemComponent false))
        (Utilities|FlowControl|Delay 7.0)
        ;;[1 1 1] Parar particulas
        (Components|Activation|ToggleActive _returnvalue)
        (Variables|Atributos|SetVida (- (Variables|Atributos|GetVida) 3.0))
        (Utilities|FlowControl|Delay 4.0)
        ;;[1 1 1] Parar animacion
        (Components|Animation|SetAnimationMode (Variables|Character|GetMesh) "AnimationBlueprint")))))

(event Input|KeyboardEvents|E
  (params (Key :type Key%20Structure :default "None"))
  ;[1 1 1] CONTROLLERS
  ;;[1 1 1] Interactuar con objetos
  (:Pressed
    ;;;[1 1 1] Objetos interactivos (clases)
    (switch string (Utilities|GetClassDisplayName (Utilities|GetClass (.HitActor (Collision|BreakHitResult (stale Custom|PlayerLookingController _outhit)))))
      (:Default
        ;;;[1 1 1] Items
        (bind _asinteractive_object (Utilities|Casting|CastToInteractiveObject (.HitActor (Collision|BreakHitResult (stale Custom|PlayerLookingController _outhit)))))
        (Default|Coger _asinteractive_object))
      (:PuertaBP_C
        (bind _aspuerta_bp (Utilities|Casting|CastToPuertaBP (.HitActor (Collision|BreakHitResult (stale Custom|PlayerLookingController _outhit)))))
        (Default|Interactuar _aspuerta_bp))
      (:ArmarioBP_C
        (bind _asarmario_bp (Utilities|Casting|CastToArmarioBP (.HitActor (Collision|BreakHitResult (stale Custom|PlayerLookingController _outhit)))))
        (Default|Interactuar _asarmario_bp))
      (:RetreteBP_C
        (bind _asretrete_bp (Utilities|Casting|CastToRetreteBP (.HitActor (Collision|BreakHitResult (stale Custom|PlayerLookingController _outhit)))))
        (Default|Interactuar _asretrete_bp)))))

(event Input|KeyboardEvents|I
  (params (Key :type Key%20Structure :default "None"))
  (bind _returnvalue (Game|GetPlayerController 0))
  (bind _inventariowidget (Variables|UI|GetInventarioWidget))
  ;[1 1 1] Mostrar Inventario
  (:Pressed
    (Widget|SetVisibility _inventariowidget "Visible")
    (Default|ObtenerInventario _inventariowidget (Variables|Inventario|GetInventario))
    (Variables|/Script/Engine.PlayerController|SetbShowMouseCursor _returnvalue true)
    (Game|SetGamePaused true)
    (Input|SetInputModeUIOnly _returnvalue 0 "DoNotLock")))

(event Input|KeyboardEvents|T
  (params (Key :type Key%20Structure :default "None"))
  ;[1 1 1] Cambiar de Jugador - Llamamos a un evento del LevelBP ya que ahi tenemos las referencias a los PJs y en cada nivel seran diferentes, sin embargo la key debe estar aqui para que no permita cambiar cuando hacemos disable input en la animacion de caida
  (:Pressed
    (Default|CallSwitchPlayer)))

(event Input|KeyboardEvents|F
  (params (Key :type Key%20Structure :default "None"))
  ;[1 1 1] CONTROLLERS
  ;;[1 1 1] Interactuar con objetos
  ;;;[1 1 1] Usar directamente
  (:Pressed
    (bind _asinteractive_object (Utilities|Casting|CastToInteractiveObject (.HitActor (Collision|BreakHitResult (stale Custom|PlayerLookingController _outhit)))))
    (switch Utilities|FlowControl|Switch|SwitchonTiposItem (.Item (Utilities|Struct|BreakItem (Variables|/Game/bin/Blueprints/InteractiveObject.InteractiveObject_C|GetItem _asinteractive_object)))
      (:NewEnumerator2
        (Default|Comer _asinteractive_object)))))

(event Input|MouseEvents|LeftMouseButton
  (params (Key :type Key%20Structure :default "None"))
  ;[1 1 1] Atacar
  (:Pressed
    (if (not (Variables|Default|GetIsAttacking?))
      (Animation|PlayAnimMontage "/Game/Modelos/Danny/Animaciones/DannyPunchAnimMontage.DannyPunchAnimMontage" 1.0 "None")
      ;;[1 1 1] Para que le de tiempo a dar un puñetazo antes de dar otro
      (Variables|Default|SetIsAttacking? true)
      (Utilities|FlowControl|Delay 0.5)
      (Variables|Default|SetIsAttacking? false))))

(fn ConstructionScript
  (|CallParentFunction))

(fn AddItem
  (params (Item :type Atributos%20Items%20Structure))
  (bind _inventario (Variables|Inventario|GetInventario))
  (bind (_value _returnvalue) (Utilities|Map|Find _inventario (.item Item)))
  ;[1 1 1] Agrega un item al inventario
  (if _returnvalue
    ;;[1 1 1] Si existe aumentamos su cantidad y reemplazamos el registro
    (bind _structout (Utilities|Struct|SetmembersinAtributosItems _value (+ (.Cantidad (Utilities|Struct|BreakAtributosItems _value)) (.cantidad Item))))
    (Utilities|Map|Add _inventario (.item Item) _structout)
    (else
      ;;[1 1 1] Si no existe lo agregamos
      (Utilities|Map|Add _inventario (.item Item) Item))))

(fn UseItem
  (params (Item :type TiposItem%20Enum :default "NewEnumerator0"))
  (bind _inventario (Variables|Inventario|GetInventario))
  (bind (_value _returnvalue) (Utilities|Map|Find _inventario Item))
  (bind _cantidad (Utilities|Struct|BreakAtributosItems _value))
  (bind _returnvalue_2 (- _cantidad 1.0))
  ;[1 1 1] La vida se coge de aqui ya que nos podemos comer objetos que no esten en el inventario
  (bind _returnvalue_3 (Utilities|GetDataTableRow "/Game/data/Tabla_Items.Tabla_Items" (Utilities|String|StringToName (Utilities|String|EnumtoString Item)))
    (:then
      (switch Utilities|FlowControl|Switch|SwitchonTiposItem Item
        (:NewEnumerator2
          ;[1 1 1] Para items curativos o venenosos
          (Variables|Atributos|SetVida (+ (Variables|Atributos|GetVida) (.vida _returnvalue_3)))
          (Audio|PlaySound2D "/Game/OST/efectos/nomNomNom.nomNomNom" 1.0 1.0 0.7 0 0)
          ;[1 1 1] Restar 1 a la cantidad de items de este tipo o borrarlo si no hay mas
          ;;[1 1 1] Solo si esta en el inventario
          (if _returnvalue
            (bind _structout (Utilities|Struct|SetmembersinAtributosItems _value _returnvalue_2))
            (if (<= _returnvalue_2 0.0)
              (Utilities|Map|Remove _inventario Item)
              (else
                (Utilities|Map|Add _inventario Item _structout)))))))))

(fn SoltarItem
  (params (Item :type TiposItem%20Enum :default "NewEnumerator0"))
  (bind _returnvalue (Math|Random|RandomUnitVector))
  (bind _inventario (Variables|Inventario|GetInventario))
  (bind _returnvalue_2 (* _returnvalue 1e+02))
  (bind _value (Utilities|Map|Find _inventario Item))
  ;[1 1 1] Direccion random en 1m a la redonda, y siempre a 10cm del suelo
  ;[1 1 1] Spawnea el item que tiramos
  (bind _returnvalue_3 (Game|SpawnActorfromClass (.clase _value) (Math|Conversions|ToTransform(Vector) (+ (Math|Vector|MakeVector (.x _returnvalue_2) (.y _returnvalue_2) -75.0) (Transformation|GetActorLocation))) "Undefined" 0 0))
  ;[1 1 1] Casteamos a clase padre para poder setear la cantidad y el tipo
  (bind _asinteractive_object (Utilities|Casting|CastToInteractiveObject _returnvalue_3))
  (Variables|/Game/bin/Blueprints/InteractiveObject.InteractiveObject_C|SetItem _asinteractive_object (Utilities|Struct|MakeItem (.item _value) (.cantidad _value)))
  ;[1 1 1] Lo quita del inventario
  (Utilities|Map|Remove _inventario Item))