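; Blueprint for the boss Hector, adding a fire trail and a second combat phase.
; A looping timer from BeginPlayBoss spawns fire bursts underfoot while it pursues alive without a montage playing.
; LifeController triggers Fase2 below half health, changing its sounds and scale.
; Phase 2 then loops on random delays until death, randomly telegraphing by sound either two enemy spawns at fixed points or eight surrounding flame explosions.
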(event Custom|LifeController
  ;[1 1 1] Control de vida para las fases
  (if (and (< (Variables|Default|GetVida) (/ (Utilities|Struct|BreakAtributosEnemies (Variables|Default|GetAtributos)) 2.0)) (not (Variables|Default|GetIsFase2?)))
    (CallFunction|Fase2)))

(event Custom|Fase2
  (bind _returnvalue (Transformation|GetActorLocation))
  ;[1 1 1] Fase 2
  (Variables|Default|SetIsFase2? true)
  ;;[1 1 1] Cuando pase a fase 2, reproducimos otros sonidos
  (Variables|Default|SetSoundCue "/Game/OST/PJs/hector/HectorSoundCueFase2.HectorSoundCueFase2")
  (Audio|PlaySound2D "/Game/OST/PJs/hector/hectorGrow.hectorGrow" 1.0 1.0 0.5 0 0)
  (Transformation|SetActorScale3D "0.300000,0.300000,0.300000")
  (Utilities|FlowControl|Delay (Math|Random|RandomFloatinRange 15.0 45.0) :!label _label)
  (if (not (Variables|Default|GetMuerto))
    ;[1 1 1] Para que sea el mismo
    (Variables|Default|SetRandomBool (Math|Random|RandomBool))
    (Audio|SpawnSoundatLocation (select (Variables|Default|GetRandomBool) "/Game/OST/efectos/godzilla.godzilla" "/Game/OST/PJs/hector/hectorCanon.hectorCanon") _returnvalue "0, 0, 0" 1.0 1.0 0.0 0 0)
    ;[1 1 1] Para que el sonido lo haga un poco antes del ataque
    (Utilities|FlowControl|Delay 1.0)
    (for _index (range 0 (select (Variables|Default|GetRandomBool) 1 7))
      (if (Variables|Default|GetRandomBool)
        (Game|SpawnActorfromClass "/Game/bin/Blueprints/Enemy.Enemy_C" (Math|Transform|MakeTransform (Utilities|Select :Index _index :Option%200 "-35911.000000,14613.000000,477.000000" :Option%201 "-35580.000000,18497.000000,477.000000") "0, 0, 0" "1,1,1") "Undefined" 0 "NewEnumerator2" 0)
        (else
          (Variables|Default|SetRandomX (Utilities|Select :Index _index :Option%200 5.4e+02 :Option%201 2.7e+02 :Option%202 0.0 :Option%203 -2.7e+02 :Option%204 -5.4e+02 :Option%205 -2.7e+02 :Option%206 0.0 :Option%207 2.7e+02))
          (Variables|Default|SetRandomY (Utilities|Select :Index _index :Option%200 0.0 :Option%201 2.7e+02 :Option%202 5.4e+02 :Option%203 2.7e+02 :Option%204 0.0 :Option%205 -5.4e+02 :Option%206 -5.4e+02 :Option%207 -2.7e+02))
          (Game|SpawnActorfromClass "/Game/Decorado/Efectos/P_FlameExplode.P_FlameExplode_C" (Math|Transform|MakeTransform (+ _returnvalue (Math|Vector|MakeVector (Variables|Default|GetRandomX) (Variables|Default|GetRandomY) -1.5e+02)) "0, 0, 0" "2.000000,2.000000,2.000000") "Undefined" 0 0))))
    (goto _label)))

(event Custom|RastroCaos
  (if (Math|Boolean|ANDBoolean (Variables|Default|GetIsPursuing?) (not (Class|AnimInstance|IsAnyMontagePlaying (Components|SkeletalMesh|GetAnimInstance (Variables|Character|GetMesh)))) (not (Variables|Default|GetMuerto)))
    ;[1 1 1] Efecto visual al caminar
    (Effects|SpawnEmitteratLocation "/Game/Decorado/Efectos/FX_Skill_RockBurst/P_RBurst_Fire_Burst_Area_01.P_RBurst_Fire_Burst_Area_01" (- (Transformation|GetActorLocation) "0, 0,150.000000"))))

(event EventBeginPlayBoss
  (Utilities|Time|SetTimerbyEvent (delegate Custom|RastroCaos) 1.5 true))

(fn ConstructionScript)