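; Neutral NPC with type-based ambient behavior, such as children playing tag or chasing a ball.
; On BeginPlay it waits for the loading screen, then mission-dependent NPCs destroy themselves if the current save's mission is past theirs.
; By type, Basket Boy follows the first SphereBP, Kid Leader patrols random offsets with random pauses, and Kid Follower chases the Kid Leader.
; Both patrol and follow are self-re-triggering AIMoveTo loops with delays.
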(event Custom|CheckMission
  (if (Variables|Default|GetMissionDependent?)
    (bind _ascustom_game_instance (Utilities|Casting|CastToCustomGameInstance (Game|GetGameInstance)))
    ;[1 1 1] Si la mision actual es superior a la que este objeto/persona deberia aparecer, lo destruimos
    (if (Utilities|IsValid (Variables|/Game/bin/Blueprints/CustomGameInstance.CustomGameInstance_C|GetCurrentSlot _ascustom_game_instance))
      (if (> (.mision (Variables|/Game/bin/Blueprints/CustomSaveGame.CustomSaveGame_C|GetMission (Variables|/Game/bin/Blueprints/CustomGameInstance.CustomGameInstance_C|GetCurrentSlot _ascustom_game_instance))) (Variables|Default|GetMision))
        (Actor|DestroyActor)))))

(event Custom|Patrullar
  (bind _returnvalue (Math|Random|RandomBool))
  ;[1 1 1] Patrullar una zona (juego pilla pilla)
  ;;[1 1 1] Va a un lado
  (AI|AIMoveTo self (+ (Transformation|GetActorLocation) (Math|Vector|MakeVector (select _returnvalue (Math|Random|RandomFloatinRange -2.7e+03 -9e+02) (Math|Random|RandomFloatinRange 9e+02 2.7e+03)) (select _returnvalue (Math|Random|RandomFloatinRange -2.7e+03 -9e+02) (Math|Random|RandomFloatinRange 9e+02 2.7e+03)) 0.0)) 0 5.0 true
    (:then
      ;;[1 1 1] Delay adicional
      (Utilities|FlowControl|Delay (Math|Random|RandomFloatinRange 0.0 15.0))
      ;;[1 1 1] Bucle
      (CallFunction|Patrullar))))

(event Custom|FollowObjetive
  (params (Objetivo :type Actor%20Object%20Reference))
  (AI|AIMoveTo self "0, 0, 0" Objetivo 5.0 false
    (:then
      ;[1 1 1] Cada medio segundo se vuelve a lanzar
      (Utilities|FlowControl|Delay 0.5)
      (CallFunction|FollowObjetive Objetivo))))

(event EventBeginPlay
  (bind _ascustom_game_instance (Utilities|Casting|CastToCustomGameInstance (Game|GetGameInstance)))
  ;[1 1 1] El mismo que pantalla de carga para que le de tiempo a cargar el savegame
  (Utilities|FlowControl|Delay (Variables|/Game/bin/Blueprints/CustomGameInstance.CustomGameInstance_C|GetLoadingScreenTime _ascustom_game_instance))
  (CallFunction|CheckMission)
  (switch Utilities|FlowControl|Switch|SwitchonNPCs (Variables|Default|GetTipo)
    (:NewEnumerator0
      (bind _outactors (Actor|GetAllActorsOfClass "/Game/StarterContent/Shapes/SphereBP.SphereBP_C"))
      (Variables|Default|SetPelota (Utilities|Array|Get(acopy) _outactors))
      (CallFunction|FollowObjetive (Variables|Default|GetPelota)))
    (:NewEnumerator3
      (CallFunction|Patrullar))
    (:NewEnumerator4
      (bind _outactors_2 (Actor|GetAllActorsOfClass "NPC_Neutral_C"))
      (bind _array_element (Utilities|Array|ForEachLoopwithBreak _outactors_2 :!label _label)
        (:LoopBody
          (if (Utilities|Enum|Equal(Enum) (Variables|NPC_Neutral_C|GetTipo _array_element) "NewEnumerator3")
            (Variables|Default|SetKidLeader _array_element)
            (goto _label Break)))
        (:Completed
          (CallFunction|FollowObjetive (Variables|Default|GetKidLeader)))))))

(fn ConstructionScript)