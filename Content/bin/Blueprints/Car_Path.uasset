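; Car path actor that lays out NPC car targets along its Path spline when play begins.
; Place_NPC_Targets loops from distance zero, spawning a Car_Destiny actor every 400 units in world space until the spline length is reached, storing each in CarTargets.
; Before spawning, it empties that array and sets old targets' lifespan to zero, which does not destroy them.
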(event Custom|Place_NPC_Targets
  (Variables|Default|SetDistance 0.0)
  (for _array_element (Variables|Default|GetCar_Targets)
    (Actor|SetLifeSpan _array_element 0.0))
  (Utilities|Array|Clear (Variables|Default|GetCar_Targets))
  (Game|SpawnActorfromClass "/Game/bin/Blueprints/Car_Destiny.Car_Destiny_C" (Math|Transform|MakeTransform (Spline|GetLocationatDistanceAlongSpline (Variables|Default|GetPath) (Variables|Default|GetDistance) "World") "0, 0, 0" "1,1,1") "Undefined" 0 0 :!label _label)
  (Utilities|Array|Add (Variables|Default|GetCar_Targets) 0)
  (Variables|Default|SetDistance (+ (Variables|Default|GetDistance) 4e+02))
  (if (< (Variables|Default|GetDistance) (Spline|GetSplineLength (Variables|Default|GetPath)))
    (goto _label)))

(event EventBeginPlay
  (CallFunction|PlaceNPCTargets))

(fn ConstructionScript)