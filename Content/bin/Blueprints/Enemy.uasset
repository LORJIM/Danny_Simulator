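; Enemy character (Hector) that patrols back and forth, chases sighted or heard players, and attacks them in melee.
; PawnSensing drives AIMoveTo pursuit into random attack montages, whose notify sphere-traces for radial damage and impulse.
; Tick sends it to the target's last position when beyond sight radius, then resumes patrol.
; Damage updates a proximity-shown health widget, low health changes looping sounds, and death ends in ragdoll with the capsule following the hips.
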(event OnSeePawn(PawnSensing)
  (params (Pawn :type Pawn%20Object%20Reference))
  (bind _self self)
  (bind _radialforce (Variables|Default|GetRadialForce))
  (bind _mesh (Variables|Character|GetMesh))
  (bind _returnvalue (Components|SkeletalMesh|GetAnimInstance _mesh))
  (bind _returnvalue_2 (Class|AnimInstance|IsAnyMontagePlaying _returnvalue))
  ;[1 1 1] Sensor de Enemigos - Perseguir Jugador
  ;;[1 1 1] Comprobar que Hector sigue vivo
  (if (not (Variables|Default|GetMuerto))
    (bind _asjugador (Utilities|Casting|CastToJugador (select (Utilities|IsValid (stale OnHearNoise(PawnSensing) Instigator)) (stale OnHearNoise(PawnSensing) Instigator) Pawn)))
    (if (Variables|/Game/bin/Blueprints/Jugador.Jugador_C|GetMuerto _asjugador)
      (bind _outactors (Actor|GetAllActorsOfClass "/Game/bin/Blueprints/Jugador.Jugador_C"))
      (bind _array_element (Utilities|Array|ForEachLoopwithBreak _outactors :!label _label)
        (:LoopBody
          ;;[1 1 1] Si esta muerto, lo que hacemos es detectar el siguiente Jugador vivo dentro del rango de escucha de Hector, y perseguir a ese
          (if (and (not (Variables|/Game/bin/Blueprints/Jugador.Jugador_C|GetMuerto _array_element)) (<= (Transformation|GetDistanceTo _array_element) (Variables|/Script/AIModule.PawnSensingComponent|GetHearingThreshold (Variables|Default|GetPawnSensing))))
            (bind _output_get (Variables|Default|SetObjetivo _array_element))
            (Variables|Default|SetIsPursuing? true)
            (if (not _returnvalue_2)
              (AI|AIMoveTo _self "0, 0, 0" _output_get 8e+01 false
                (:then
                  (goto _label Break))
                (:OnSuccess
                  ;;[1 1 1] Si consigue llegar a su objetivo, ataca
                  (Variables|Default|SetIsPursuing? false :!label _label_2)
                  ;[1 1 1] Para que coincida en ambos select
                  (bind _output_get_2 (Variables|Default|SetAttackAnimation (Math|Random|RandomInteger 3)))
                  (Animation|Montage|PlayMontage _mesh (Utilities|Select :Index _output_get_2 :Option%200 "/Game/Modelos/HECTOR/Animaciones/Mutant_Punch_Montage.Mutant_Punch_Montage" :Option%201 "/Game/Modelos/HECTOR/Animaciones/Kicking_Montage.Kicking_Montage" :Option%202 "/Game/Modelos/HECTOR/Animaciones/Zombie_Attack_Montage.Zombie_Attack_Montage")
                    (:OnNotifyBegin
                      ;[1 1 1] Golpear
                      ;;[1 1 1] Esfera alrededor del socket donde se produce el golpe
                      (bind _returnvalue_3 (Collision|SphereTraceByChannel (Transformation|GetSocketLocation (Variables|Character|GetMesh) (Utilities|Select :Index _output_get_2 :Option%200 "RightHandSocket" :Option%201 "RightFeetSocket" :Option%202 "RightHandSocket")) (Transformation|GetSocketLocation (Variables|Character|GetMesh) (Utilities|Select :Index _output_get_2 :Option%200 "RightHandSocket" :Option%201 "RightFeetSocket" :Option%202 "RightHandSocket")) 5e+01 "TraceTypeQuery1" false 0 "None"))
                      ;;[1 1 1] Si golpea
                      (if _returnvalue_3
                        ;;[1 1 1] Rebote
                        (Class|RadialForceComponent|FireImpulse _radialforce)
                        ;;[1 1 1] Aplica damage a los que entren en el radio
                        (Game|Damage|ApplyRadialDamage (Variables|Default|GetAtaque) (Transformation|GetSocketLocation (Variables|Character|GetMesh) (Utilities|Select :Index _output_get_2 :Option%200 "RightHandSocket" :Option%201 "RightFeetSocket" :Option%202 "RightHandSocket")) (Variables|/Script/Engine.RadialForceComponent|GetRadius _radialforce) 0 0 _self 0 false "ECC_WorldDynamic")
                        ;;[1 1 1] Sonido
                        (Audio|SpawnSoundatLocation "/Game/OST/efectos/golpe.golpe" (Transformation|GetSocketLocation (Variables|Character|GetMesh) (Utilities|Select :Index _output_get_2 :Option%200 "RightHandSocket" :Option%201 "RightFeetSocket" :Option%202 "RightHandSocket")) "0, 0, 0" 0.5 1.0 0.0 0 0)
                        ;;[1 1 1] Efecto visual
                        (Effects|SpawnEmitteratLocation "/Game/Decorado/Efectos/FX_Skill_Leap/P_Skill_Leap_Poison_Impact_Impact.P_Skill_Leap_Poison_Impact_Impact" (Transformation|GetSocketLocation (Variables|Character|GetMesh) (Utilities|Select :Index _output_get_2 :Option%200 "RightHandSocket" :Option%201 "RightFeetSocket" :Option%202 "RightHandSocket"))))))))))))
      (else
        (bind _output_get_3 (Variables|Default|SetObjetivo _asjugador))
        (Variables|Default|SetIsPursuing? true)
        (if (not _returnvalue_2)
          ;;[1 1 1] Si esta vivo pues lo perseguimos
          (AI|AIMoveTo _self "0, 0, 0" _output_get_3 8e+01 false
            (:OnSuccess
              (goto _label_2))))))))

(event OnComponentBeginOverlap(SphereCollision)
  (params (OverlappedComponent :type Primitive%20Component%20Object%20Reference) (OtherActor :type Actor%20Object%20Reference) (OtherComp :type Primitive%20Component%20Object%20Reference) (OtherBodyIndex :type Integer) (bFromSweep :type Boolean) (SweepResult :type Hit%20Result%20Structure%20%28by%20ref%29))
  ;[1 1 1] Mostrar/Ocultar barra de salud y nombre cuando nos acercamos
  (Utilities|Casting|CastToJugador OtherActor)
  (Rendering|SetVisibility (Variables|Default|GetWidget) true false))

(event OnHearNoise(PawnSensing)
  (params (Instigator :type Pawn%20Object%20Reference) (Location :type Vector%20%28by%20ref%29 :default "0, 0, 0") (Volume :type Float%20%28single-precision%29))
  (bind _self self)
  (bind _radialforce (Variables|Default|GetRadialForce))
  (bind _mesh (Variables|Character|GetMesh))
  (bind _returnvalue (Components|SkeletalMesh|GetAnimInstance _mesh))
  (bind _returnvalue_2 (Class|AnimInstance|IsAnyMontagePlaying _returnvalue))
  ;[1 1 1] Sensor de Enemigos - Perseguir Jugador
  ;;[1 1 1] Comprobar que Hector sigue vivo
  (if (not (Variables|Default|GetMuerto))
    (bind _asjugador (Utilities|Casting|CastToJugador (select (Utilities|IsValid Instigator) Instigator (stale OnSeePawn(PawnSensing) Pawn))))
    (if (Variables|/Game/bin/Blueprints/Jugador.Jugador_C|GetMuerto _asjugador)
      (bind _outactors (Actor|GetAllActorsOfClass "/Game/bin/Blueprints/Jugador.Jugador_C"))
      (bind _array_element (Utilities|Array|ForEachLoopwithBreak _outactors :!label _label)
        (:LoopBody
          ;;[1 1 1] Si esta muerto, lo que hacemos es detectar el siguiente Jugador vivo dentro del rango de escucha de Hector, y perseguir a ese
          (if (and (not (Variables|/Game/bin/Blueprints/Jugador.Jugador_C|GetMuerto _array_element)) (<= (Transformation|GetDistanceTo _array_element) (Variables|/Script/AIModule.PawnSensingComponent|GetHearingThreshold (Variables|Default|GetPawnSensing))))
            (bind _output_get (Variables|Default|SetObjetivo _array_element))
            (Variables|Default|SetIsPursuing? true)
            (if (not _returnvalue_2)
              (AI|AIMoveTo _self "0, 0, 0" _output_get 8e+01 false
                (:then
                  (goto _label Break))
                (:OnSuccess
                  ;;[1 1 1] Si consigue llegar a su objetivo, ataca
                  (Variables|Default|SetIsPursuing? false :!label _label_2)
                  ;[1 1 1] Para que coincida en ambos select
                  (bind _output_get_2 (Variables|Default|SetAttackAnimation (Math|Random|RandomInteger 3)))
                  (Animation|Montage|PlayMontage _mesh (Utilities|Select :Index _output_get_2 :Option%200 "/Game/Modelos/HECTOR/Animaciones/Mutant_Punch_Montage.Mutant_Punch_Montage" :Option%201 "/Game/Modelos/HECTOR/Animaciones/Kicking_Montage.Kicking_Montage" :Option%202 "/Game/Modelos/HECTOR/Animaciones/Zombie_Attack_Montage.Zombie_Attack_Montage")
                    (:OnNotifyBegin
                      ;[1 1 1] Golpear
                      ;;[1 1 1] Esfera alrededor del socket donde se produce el golpe
                      (bind _returnvalue_3 (Collision|SphereTraceByChannel (Transformation|GetSocketLocation (Variables|Character|GetMesh) (Utilities|Select :Index _output_get_2 :Option%200 "RightHandSocket" :Option%201 "RightFeetSocket" :Option%202 "RightHandSocket")) (Transformation|GetSocketLocation (Variables|Character|GetMesh) (Utilities|Select :Index _output_get_2 :Option%200 "RightHandSocket" :Option%201 "RightFeetSocket" :Option%202 "RightHandSocket")) 5e+01 "TraceTypeQuery1" false 0 "None"))
                      ;;[1 1 1] Si golpea
                      (if _returnvalue_3
                        ;;[1 1 1] Rebote
                        (Class|RadialForceComponent|FireImpulse _radialforce)
                        ;;[1 1 1] Aplica damage a los que entren en el radio
                        (Game|Damage|ApplyRadialDamage (Variables|Default|GetAtaque) (Transformation|GetSocketLocation (Variables|Character|GetMesh) (Utilities|Select :Index _output_get_2 :Option%200 "RightHandSocket" :Option%201 "RightFeetSocket" :Option%202 "RightHandSocket")) (Variables|/Script/Engine.RadialForceComponent|GetRadius _radialforce) 0 0 _self 0 false "ECC_WorldDynamic")
                        ;;[1 1 1] Sonido
                        (Audio|SpawnSoundatLocation "/Game/OST/efectos/golpe.golpe" (Transformation|GetSocketLocation (Variables|Character|GetMesh) (Utilities|Select :Index _output_get_2 :Option%200 "RightHandSocket" :Option%201 "RightFeetSocket" :Option%202 "RightHandSocket")) "0, 0, 0" 0.5 1.0 0.0 0 0)
                        ;;[1 1 1] Efecto visual
                        (Effects|SpawnEmitteratLocation "/Game/Decorado/Efectos/FX_Skill_Leap/P_Skill_Leap_Poison_Impact_Impact.P_Skill_Leap_Poison_Impact_Impact" (Transformation|GetSocketLocation (Variables|Character|GetMesh) (Utilities|Select :Index _output_get_2 :Option%200 "RightHandSocket" :Option%201 "RightFeetSocket" :Option%202 "RightHandSocket"))))))))))))
      (else
        (bind _output_get_3 (Variables|Default|SetObjetivo _asjugador))
        (Variables|Default|SetIsPursuing? true)
        (if (not _returnvalue_2)
          ;;[1 1 1] Si esta vivo pues lo perseguimos
          (AI|AIMoveTo _self "0, 0, 0" _output_get_3 8e+01 false
            (:OnSuccess
              (goto _label_2))))))))

(event OnComponentEndOverlap(SphereCollision)
  (params (OverlappedComponent :type Primitive%20Component%20Object%20Reference) (OtherActor :type Actor%20Object%20Reference) (OtherComp :type Primitive%20Component%20Object%20Reference) (OtherBodyIndex :type Integer))
  ;[1 1 1] Mostrar/Ocultar barra de salud y nombre cuando nos acercamos
  (Utilities|Casting|CastToJugador OtherActor)
  (Rendering|SetVisibility (Variables|Default|GetWidget) false false))

(event Custom|Patrullar
  (bind _returnvalue (Transformation|GetActorLocation))
  (bind _self self)
  (bind _mesh (Variables|Character|GetMesh))
  ;[1 1 1] Patrullar una zona
  (if (Math|Boolean|NANDBoolean (Variables|Default|GetIsPursuing?) (Variables|Default|GetMuerto) (Class|AnimInstance|IsAnyMontagePlaying (Components|SkeletalMesh|GetAnimInstance (Variables|Character|GetMesh))))
    ;;[1 1 1] Para que coincida en ambos select
    (bind _output_get (Variables|Default|SetPatrolAnimation (Math|Random|RandomInteger 3)))
    (Utilities|FlowControl|FlipFlop
      (:A
        ;;[1 1 1] Va a un lado
        (AI|AIMoveTo _self (- _returnvalue "0,900.000000, 0") 0 5.0 false
          (:OnSuccess
            _)
          (:OnFail
            _)))
      (:B
        ;;[1 1 1] Va a otro
        (AI|AIMoveTo _self (+ _returnvalue "0,900.000000, 0") 0 5.0 false
          (:OnSuccess
            _)
          (:OnFail
            _))))
    (Components|Animation|PlayAnimation _mesh (Utilities|Select :Index _output_get :Option%200 "/Game/Modelos/HECTOR/Animaciones/Kicking.Kicking" :Option%201 "/Game/Modelos/HECTOR/Animaciones/Mutant_Roaring.Mutant_Roaring" :Option%202 "/Game/Modelos/HECTOR/Animaciones/Standing_Yell.Standing_Yell") false)
    ;;[1 1 1] Tiempo ejecutando anim
    (Utilities|FlowControl|Delay (Utilities|Select :Index _output_get :Option%200 2.1 :Option%201 5.4 :Option%202 3.7))
    (Components|Animation|SetAnimationMode _mesh "AnimationBlueprint")
    ;;[1 1 1] Delay adicional
    (Utilities|FlowControl|Delay (Math|Random|RandomFloatinRange 0.0 15.0))
    ;;[1 1 1] Bucle
    (CallFunction|Patrullar)))

(event Custom|RagdollCapsuleController
  ;[1 1 1] Mantener capsula cuando entramos en Ragdoll
  (if (Variables|Default|GetRagdoll)
    (Transformation|SetWorldLocation (Variables|Collision|GetCapsuleComponent) (+ (Transformation|GetSocketLocation (Variables|Character|GetMesh) "Hips") "0, 0,700.000000") false false)))

(event Custom|Sonido
  ;[1 1 1] Rastro Destruccion - Reproducir Sonidos de Hector - Patrullar nada mas empezar
  ;;[1 1 1] Cuando pase a fase 2, reproducimos otros sonidos
  (if (not (Variables|Default|GetMuerto))
    (bind _returnvalue (Audio|SpawnSoundatLocation (select (< (Variables|Default|GetVida) (/ (.Vida (Utilities|GetClassDefaults "/Game/bin/Blueprints/Hector.Hector_C")) 2.0)) "/Game/OST/PJs/hector/HectorSoundCueFase2.HectorSoundCueFase2" "/Game/OST/PJs/hector/HectorSoundCue.HectorSoundCue") (Transformation|GetActorLocation) "0, 0, 0" 1.0 1.0 0.0 0 0))
    ;;[1 1 1] Para poder pararlo cuando muera
    (Variables|Components|SetCurrentSound _returnvalue)
    (Utilities|FlowControl|Delay 12.5)
    (CallFunction|Sonido)))

(event Custom|ControllerObjetivo
  (bind _objetivo (Variables|Default|GetObjetivo))
  ;[1 1 1] Si nos persigue pero ya estamos fuera de su radio de vista, este controller hace que hector vaya al ultimo sitio donde hemos estado. Si consigue llegar antes de volvernos a ver (lo cual haria que fallara este AIMoveTo al desviar el rumbo), pues le diremos que comience a patrullar de nuevo
  (if (and (Variables|Default|GetIsPursuing?) (> (Transformation|GetDistanceTo _objetivo) (Variables|/Script/AIModule.PawnSensingComponent|GetSightRadius (Variables|Default|GetPawnSensing))))
    ;;[1 1 1] Para que no ejecute este controller infinitas veces
    (Variables|Default|SetIsPursuing? false)
    (AI|AIMoveTo self (Transformation|GetActorLocation _objetivo) 0 1.0 false
      (:OnSuccess
        (CallFunction|Patrullar)))))

(event Custom|RastroCaos
  ;[1 1 1] Rastro Destruccion - Reproducir Sonidos de Hector - Patrullar nada mas empezar
  (if (Math|Boolean|ANDBoolean (Variables|Default|GetIsPursuing?) (not (Class|AnimInstance|IsAnyMontagePlaying (Components|SkeletalMesh|GetAnimInstance (Variables|Character|GetMesh)))) (not (Variables|Default|GetMuerto)))
    ;[1 1 1] Efecto visual al caminar
    (Effects|SpawnEmitteratLocation "/Game/Decorado/Efectos/FX_Skill_RockBurst/P_RBurst_Fire_Burst_Area_01.P_RBurst_Fire_Burst_Area_01" (- (Transformation|GetActorLocation) "0, 0,150.000000"))))

(event EventBeginPlay
  ;[1 1 1] Rastro Destruccion - Reproducir Sonidos de Hector - Patrullar nada mas empezar
  (bind _asnpc (Utilities|Casting|CastToNPC (UserInterface|GetUserWidgetObject (Variables|Default|GetWidget))))
  (bind _output_get (Variables|Default|SetHeadWidget _asnpc))
  (Default|SetValues _output_get (Variables|Default|GetVida) (Utilities|Text|ToText(String) (Utilities|String|EnumtoString (Variables|Default|GetTipo))))
  (CallFunction|Sonido)
  (CallFunction|Patrullar)
  (Utilities|Time|SetTimerbyEvent (delegate Custom|RastroCaos) 1.5 true))

(event EventTick
  (params (DeltaSeconds :type Float%20%28single-precision%29))
  ;[1 1 1] Controller para que deje de perseguir cuando nos pierda de vista
  (CallFunction|ControllerObjetivo)
  (CallFunction|RagdollCapsuleController))

(event Game|Damage|EventAnyDamage
  (params (Damage :type Float%20%28single-precision%29) (DamageType :type Damage%20Type%20Object%20Reference) (InstigatedBy :type Controller%20Object%20Reference) (DamageCauser :type Actor%20Object%20Reference))
  (bind _returnvalue (Transformation|GetActorLocation))
  (bind _currentsound (Variables|Components|GetCurrentSound))
  (bind _mesh (Variables|Character|GetMesh))
  ;[1 1 1] Recibir Damage y Morir
  (bind _output_get (Variables|Default|SetVida (- (Variables|Default|GetVida) Damage)))
  (Variables|/Game/UI/NPC.NPC_C|SetVida (Variables|Default|GetHeadWidget) _output_get)
  (if (and (<= _output_get 0.0) (not (Variables|Default|GetMuerto)))
    ;;[1 1 1] Muerte
    (Variables|Default|SetMuerto true)
    (if (Utilities|IsValid _currentsound)
      ;;;[1 1 1] Parar audio actual si lo hay
      (Audio|Components|Audio|Stop _currentsound))
    (Audio|SpawnSoundatLocation "/Game/OST/PJs/hector/HectorDeathIngame.HectorDeathIngame" _returnvalue "0, 0, 0" 0.5 1.0 0.0 0 0)
    ;;[1 1 1] Lo detenemos
    (Pawn|Components|CharacterMovement|DisableMovement (Variables|Character|GetCharacterMovement))
    ;;[1 1 1] Efecto visual
    (Effects|SpawnEmitteratLocation "/Game/Decorado/Efectos/FX_Monsters/FX_Monster_Deaths/P_Monster_Death_Large_Fire.P_Monster_Death_Large_Fire" (- _returnvalue "0, 0,150.000000"))
    (Animation|Montage|PlayMontage _mesh "/Game/Modelos/HECTOR/Animaciones/Standing_React_Death_Backward_Montage.Standing_React_Death_Backward_Montage"
      (:OnCompleted
        (Class|SkeletalMeshComponent|SetAllBodiesBelowSimulatePhysics _mesh (Utilities|Name|MakeLiteralName "hips") true true)
        (Variables|Default|SetRagdoll true)))
    (else
      ;;[1 1 1] Damage - Efecto Visual
      (Effects|SpawnEmitteratLocation "/Game/Decorado/Efectos/FX_Monsters/FX_Monster_Bear/Impact/P_Bear_Swing_Impact_Poison.P_Bear_Swing_Impact_Poison" _returnvalue))))

(fn ConstructionScript)