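; Pato_NPC is an NPC Blueprint that patrols back and forth along the Y axis from BeginPlay.
; A FlipFlop alternates AI MoveTo destinations 900 units to either side of the current location.
; On success or failure it waits a random whole number of seconds, to desynchronize multiple instances, then calls Patrullar again to loop.
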(event Custom|Patrullar
  (bind _returnvalue (Transformation|GetActorLocation))
  (bind _self self)
  ;[1 1 1] Patrullar una zona
  (Utilities|FlowControl|FlipFlop
    (:A
      ;;[1 1 1] Va a un lado
      (AI|AIMoveTo _self (- _returnvalue "0,900.000000, 0") 0 5.0 false
        (:OnSuccess
          _)
        (:OnFail
          _)))
    (:B
      ;;[1 1 1] Va a otro
      (AI|AIMoveTo _self (+ _returnvalue "0,900.000000, 0") 0 5.0 false
        (:OnSuccess
          _)
        (:OnFail
          _))))
  ;;[1 1 1] Tiempo parado
  (Utilities|FlowControl|Delay (Math|Conversions|ToFloat(Integer) (Math|Random|RandomInteger 15)))
  ;;[1 1 1] Bucle
  (CallFunction|Patrullar))

(event EventBeginPlay
  ;[1 1 1] Trigger inicial
  (CallFunction|Patrullar))

(fn ConstructionScript)