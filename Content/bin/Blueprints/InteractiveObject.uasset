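; InteractiveObject is a base Blueprint for interactive world objects, especially items the player can take or consume.
; Coger adds its Atributos to the Jugador's inventory, while Comer uses the item on the spot; both then destroy the actor.
; An unfinished height-based grab animation compares the actor's Z with itself, so it always picks Picking_Up_Object.
; The sequence that calls it and restores the animation Blueprint is disconnected.
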(event Custom|Comer
  (bind _asjugador (Utilities|Casting|CastToJugador (Game|Player|GetPlayerPawn 0)))
  ;[1 1 1] Comer
  (Default|UseItem _asjugador (.Item (Utilities|Struct|BreakAtributosItems (Variables|Default|GetAtributos))))
  ;[1 1 1] Desaparece
  (Actor|DestroyActor))

(event Custom|Coger
  (bind _asjugador (Utilities|Casting|CastToJugador (Game|Player|GetPlayerPawn 0)))
  ;[1 1 1] Agregar al inventario
  (Default|AddItem _asjugador (Variables|Default|GetAtributos))
  ;[1 1 1] Desaparece
  (Actor|DestroyActor))

(event Custom|AnimacionAgarrar
  ;[1 1 1] PDTE DE DESARROLLO - ANIMACION DE COGER SEGUN ALTURA TIENE ALGUNOS BUGS
  (bind _asjugador (Utilities|Casting|CastToJugador (Game|Player|GetPlayerPawn 0)))
  (if (< (- (.z (Transformation|GetActorLocation)) 5e+01) (.z (Transformation|GetActorLocation)))
    (Components|Animation|PlayAnimation (Variables|/Script/Engine.Character|GetMesh _asjugador) "/Game/Modelos/Danny/Animaciones/Picking_Up_Object.Picking_Up_Object" false)
    (else
      (Components|Animation|PlayAnimation (Variables|/Script/Engine.Character|GetMesh _asjugador) "/Game/Modelos/Danny/Animaciones/Lifting.Lifting" false))))

(fn ConstructionScript)