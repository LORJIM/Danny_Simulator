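; NPC_Path is a spline-based actor that lays out NPC_Destiny target actors along its Path spline when play begins.
; Place_NPC_Targets sets each tracked target's lifespan to zero, which does not destroy it, and clears the NPCTargets array.
; It then loops from the spline's start, spawning targets at a fixed distance interval in world space and storing them in the array.
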(event Custom|Place_NPC_Targets
  (Variables|Default|SetDistance 0.0)
  (for _array_element (Variables|Default|GetNPC_Targets)
    (Actor|SetLifeSpan _array_element 0.0))
  (Utilities|Array|Clear (Variables|Default|GetNPC_Targets))
  (bind _returnvalue (Game|SpawnActorfromClass "/Game/bin/Blueprints/NPC_Destiny.NPC_Destiny_C" (Math|Transform|MakeTransform (Spline|GetLocationatDistanceAlongSpline (Variables|Default|GetPath) (Variables|Default|GetDistance) "World") "0, 0, 0" "1,1,1") "Undefined" 0 0 :!label _label))
  (Utilities|Array|Add (Variables|Default|GetNPC_Targets) _returnvalue)
  (Variables|Default|SetDistance (+ (Variables|Default|GetDistance) 4e+02))
  (if (< (Variables|Default|GetDistance) (Spline|GetSplineLength (Variables|Default|GetPath)))
    (goto _label)))

(event EventBeginPlay
  (CallFunction|PlaceNPCTargets))

(fn ConstructionScript)