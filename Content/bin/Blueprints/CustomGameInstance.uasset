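; Custom Game Instance that handles saving and loading player state and the current level through CustomSaveGame slots.
; SaveGame records each Jugador's transform, adds the actor itself to a map keyed by Tipo, and stores the level name.
; LoadGame caches the slot in CurrentSlot and opens its level.
; LoadData, a separate event not called here, copies stats and transforms from CurrentSlot onto matching Jugador actors.
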(event Custom|SaveGame
  (params (SlotFileName :type String) (SlotName :type Text))
  ;[1 1 1] Procesamiento - Guardar variables
  (bind _returnvalue (SaveGame|CreateSaveGameObject "/Game/bin/Blueprints/CustomSaveGame.CustomSaveGame_C"))
  (Variables|/Game/bin/Blueprints/CustomSaveGame.CustomSaveGame_C|SetNombreSaveGame _returnvalue SlotName)
  (bind _outactors (Actor|GetAllActorsOfClass "/Game/bin/Blueprints/Jugador.Jugador_C"))
  (for _array_element _outactors
    (Variables|/Game/bin/Blueprints/Jugador.Jugador_C|SetLocation _array_element (Transformation|GetActorTransform _array_element))
    (Development|PrintString (Utilities|String|ToString(Float) (Variables|/Game/bin/Blueprints/Jugador.Jugador_C|GetVida _array_element)))
    (Utilities|Map|Add (Variables|/Game/bin/Blueprints/CustomSaveGame.CustomSaveGame_C|GetJugadores _returnvalue) (Variables|/Game/bin/Blueprints/Jugador.Jugador_C|GetTipo _array_element) _array_element))
  (bind _returnvalue_2 (Game|GetCurrentLevelName true))
  (Variables|/Game/bin/Blueprints/CustomSaveGame.CustomSaveGame_C|SetNivel _returnvalue (Utilities|String|StringToName _returnvalue_2))
  (SaveGame|SaveGametoSlot _returnvalue SlotFileName))

(event Custom|LoadData
  ;[1 1 1] Procesamiento - Cargar variables
  (bind _outactors (Actor|GetAllActorsOfClass "/Game/bin/Blueprints/Jugador.Jugador_C"))
  (for _array_element _outactors
    (Development|PrintString (Utilities|String|EnumtoString (Variables|/Game/bin/Blueprints/Jugador.Jugador_C|GetTipo (.Value (Utilities|Map|Find (Variables|/Game/bin/Blueprints/CustomSaveGame.CustomSaveGame_C|GetJugadores (Variables|Default|GetCurrentSlot)) (Variables|/Game/bin/Blueprints/Jugador.Jugador_C|GetTipo _array_element))))))
    (if (.ReturnValue (Utilities|Map|Find (Variables|/Game/bin/Blueprints/CustomSaveGame.CustomSaveGame_C|GetJugadores (Variables|Default|GetCurrentSlot)) (Variables|/Game/bin/Blueprints/Jugador.Jugador_C|GetTipo _array_element)))
      (Variables|/Game/bin/Blueprints/Jugador.Jugador_C|SetVelocidad _array_element (Variables|/Game/bin/Blueprints/Jugador.Jugador_C|GetVelocidad (.Value (Utilities|Map|Find (Variables|/Game/bin/Blueprints/CustomSaveGame.CustomSaveGame_C|GetJugadores (Variables|Default|GetCurrentSlot)) (Variables|/Game/bin/Blueprints/Jugador.Jugador_C|GetTipo _array_element)))))
      (Variables|/Game/bin/Blueprints/Jugador.Jugador_C|SetDefensa _array_element (Variables|/Game/bin/Blueprints/Jugador.Jugador_C|GetDefensa (.Value (Utilities|Map|Find (Variables|/Game/bin/Blueprints/CustomSaveGame.CustomSaveGame_C|GetJugadores (Variables|Default|GetCurrentSlot)) (Variables|/Game/bin/Blueprints/Jugador.Jugador_C|GetTipo _array_element)))))
      (Variables|/Game/bin/Blueprints/Jugador.Jugador_C|SetAtaque _array_element (Variables|/Game/bin/Blueprints/Jugador.Jugador_C|GetAtaque (.Value (Utilities|Map|Find (Variables|/Game/bin/Blueprints/CustomSaveGame.CustomSaveGame_C|GetJugadores (Variables|Default|GetCurrentSlot)) (Variables|/Game/bin/Blueprints/Jugador.Jugador_C|GetTipo _array_element)))))
      (Variables|/Game/bin/Blueprints/Jugador.Jugador_C|SetVida _array_element (Variables|/Game/bin/Blueprints/Jugador.Jugador_C|GetVida (.Value (Utilities|Map|Find (Variables|/Game/bin/Blueprints/CustomSaveGame.CustomSaveGame_C|GetJugadores (Variables|Default|GetCurrentSlot)) (Variables|/Game/bin/Blueprints/Jugador.Jugador_C|GetTipo _array_element)))))
      (Variables|/Game/bin/Blueprints/Jugador.Jugador_C|SetVejiga _array_element (Variables|/Game/bin/Blueprints/Jugador.Jugador_C|GetVejiga (.Value (Utilities|Map|Find (Variables|/Game/bin/Blueprints/CustomSaveGame.CustomSaveGame_C|GetJugadores (Variables|Default|GetCurrentSlot)) (Variables|/Game/bin/Blueprints/Jugador.Jugador_C|GetTipo _array_element)))))
      (Transformation|SetActorTransform _array_element (Variables|/Game/bin/Blueprints/Jugador.Jugador_C|GetLocation (.Value (Utilities|Map|Find (Variables|/Game/bin/Blueprints/CustomSaveGame.CustomSaveGame_C|GetJugadores (Variables|Default|GetCurrentSlot)) (Variables|/Game/bin/Blueprints/Jugador.Jugador_C|GetTipo _array_element))))))))

(event Custom|LoadGame
  (params (SlotFileName :type String))
  (bind _returnvalue (SaveGame|DoesSaveGameExist SlotFileName))
  (if _returnvalue
    (bind _returnvalue_2 (SaveGame|LoadGamefromSlot SlotFileName))
    (bind _ascustom_save_game (Utilities|Casting|CastToCustomSaveGame _returnvalue_2))
    (Development|PrintString (Utilities|String|ToString(Transform) (Variables|/Game/bin/Blueprints/Jugador.Jugador_C|GetLocation (.Value (Utilities|Map|Find (Variables|/Game/bin/Blueprints/CustomSaveGame.CustomSaveGame_C|GetJugadores _ascustom_save_game) "NewEnumerator1")))))
    (bind _output_get (Variables|Default|SetCurrentSlot _ascustom_save_game))
    (Game|OpenLevel(byName) (Variables|/Game/bin/Blueprints/CustomSaveGame.CustomSaveGame_C|GetNivel _output_get))
    (else
      (Development|PrintString "NO HAY NADA GUARDADO AQUI ZOQUETE"))))