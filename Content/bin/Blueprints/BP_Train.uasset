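; BP_Train is a train actor that shuttles back and forth along a rail spline, pausing at stations.
; A timeline moves it by distance along the spline, with play rate derived from the seconds per line, and flips direction on finishing.
; Stop and start timelines scale that play rate, with a timer restarting the train after a short wait.
; Front and back triggers stop it for tagged obstacles in its direction of travel.
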(event OnComponentBeginOverlap(StationDetectionTrigger)
  (params (OverlappedComponent :type Primitive%20Component%20Object%20Reference) (OtherActor :type Actor%20Object%20Reference) (OtherComp :type Primitive%20Component%20Object%20Reference) (OtherBodyIndex :type Integer) (bFromSweep :type Boolean) (SweepResult :type Hit%20Result%20Structure%20%28by%20ref%29))
  ;[1 1 1] Stop Train
  (if (Actor|ActorHasTag OtherActor "Station")
    (bind _stoptrainspeedalpha (Timeline|StopTimeline PlayFromStart)
      (:Update
        (Components|Timeline|SetPlayRate (Variables|Default|GetFollowRailTimeline) (Math|Float|Lerp 0.0 (Variables|Default|GetSpeedScalar) _stoptrainspeedalpha))
        ;[1 1 1] Wait and restart train
        (Utilities|Time|SetTimerbyEvent (delegate Custom|OnTrainStopFinished) 3.0)))))

(event OnComponentBeginOverlap(FrontEmergencyStopDetectionTrigger)
  (params (OverlappedComponent :type Primitive%20Component%20Object%20Reference) (OtherActor :type Actor%20Object%20Reference) (OtherComp :type Primitive%20Component%20Object%20Reference) (OtherBodyIndex :type Integer) (bFromSweep :type Boolean) (SweepResult :type Hit%20Result%20Structure%20%28by%20ref%29))
  ;[1 1 1] Emergency break and restart
  (if (Variables|Default|GetGoingForward)
    (if (Actor|ActorHasTag OtherActor "Obstacle")
      ;[1 1 1] Stop Train
      (bind _stoptrainspeedalpha (Timeline|StopTimeline PlayFromStart)
        (:Update
          (Components|Timeline|SetPlayRate (Variables|Default|GetFollowRailTimeline) (Math|Float|Lerp 0.0 (Variables|Default|GetSpeedScalar) _stoptrainspeedalpha))
          ;[1 1 1] Wait and restart train
          (Utilities|Time|SetTimerbyEvent (delegate Custom|OnTrainStopFinished) 3.0))))))

(event OnComponentBeginOverlap(BackEmergencyStopDetectionTrigger)
  (params (OverlappedComponent :type Primitive%20Component%20Object%20Reference) (OtherActor :type Actor%20Object%20Reference) (OtherComp :type Primitive%20Component%20Object%20Reference) (OtherBodyIndex :type Integer) (bFromSweep :type Boolean) (SweepResult :type Hit%20Result%20Structure%20%28by%20ref%29))
  ;[1 1 1] Emergency break and restart
  (if (not (Variables|Default|GetGoingForward))
    (if (Actor|ActorHasTag OtherActor "Obstacle")
      ;[1 1 1] Stop Train
      (bind _stoptrainspeedalpha (Timeline|StopTimeline PlayFromStart)
        (:Update
          (Components|Timeline|SetPlayRate (Variables|Default|GetFollowRailTimeline) (Math|Float|Lerp 0.0 (Variables|Default|GetSpeedScalar) _stoptrainspeedalpha))
          ;[1 1 1] Wait and restart train
          (Utilities|Time|SetTimerbyEvent (delegate Custom|OnTrainStopFinished) 3.0))))))

(event Custom|OnTrainStopFinished
  ;[1 1 1] Wait and restart train
  (bind _stoptrainspeedalpha (Timeline|StartTimeline PlayFromStart)
    (:Update
      (Components|Timeline|SetPlayRate (Variables|Default|GetFollowRailTimeline) (Math|Float|Lerp 0.0 (Variables|Default|GetSpeedScalar) _stoptrainspeedalpha)))))

(event Custom|OnTrainStopDelayed
  ;[1 1 1] Todo. trigger when a pause is needed
  (Utilities|Time|SetTimerbyEvent (delegate Custom|OnTrainStopFinished) 3.0)
  ;[1 1 1] Wait and restart train
  (bind _stoptrainspeedalpha (Timeline|StartTimeline Stop)
    (:Update
      (Components|Timeline|SetPlayRate (Variables|Default|GetFollowRailTimeline) (Math|Float|Lerp 0.0 (Variables|Default|GetSpeedScalar) _stoptrainspeedalpha)))))

(event EventBeginPlay
  ;[1 1 1] Train movement
  (bind _output_get (Variables|Default|SetSpeedScalar (Math|Float|SafeDivide 1.0 (Variables|Default|GetSeconds%20to%20complete%20a%20line))))
  (Components|Timeline|SetPlayRate (Variables|Default|GetFollowRailTimeline) _output_get)
  (if (Variables|Default|GetGoingForward) :!label _label
    (bind _raildistancealpha (Timeline|FollowRailTimeline Play)
      (:Update
        (Transformation|SetActorTransform (Spline|GetTransformatDistanceAlongSpline (Variables|/Game/bin/Blueprints/BP_RailSpline.BP_RailSpline_C|GetTrack (Variables|Default|GetRailSpline)) (Math|Float|Lerp 0.0 (Spline|GetSplineLength (Variables|/Game/bin/Blueprints/BP_RailSpline.BP_RailSpline_C|GetTrack (Variables|Default|GetRailSpline))) _raildistancealpha) "World" true)))
      (:Finished
        (Variables|Default|SetGoingForward (not (Variables|Default|GetGoingForward)))
        (goto _label)))
    (else
      (Timeline|FollowRailTimeline Reverse))))

(fn ConstructionScript)

(fn StopTrain)