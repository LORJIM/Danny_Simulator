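; AI controller for a pedestrian that wanders endlessly between targets, starting 40 seconds after BeginPlay.
; It sphere-traces ahead of the pawn on a custom object type, ignoring the current target, and widens the radius until something is hit.
; It moves to a random reachable point near a random hit, then searches again on success or after a brief delay on failure.
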(event Custom|Go_to
  (params (Target :type Vector))
  (AI|AIMoveTo 0 Target 0 1e+02 false
    (:OnSuccess
      _)
    (:OnFail
      (Utilities|FlowControl|Delay 0.2)))
  (CallFunction|NextTarget))

(event EventBeginPlay
  (Utilities|FlowControl|Delay 4e+01)
  (CallFunction|NextTarget))

(fn ConstructionScript)

(event Custom|Next_Target
  (bind _returnvalue (Pawn|GetControlledPawn))
  (bind _returnvalue_2 (Transformation|GetActorLocation _returnvalue))
  (bind _returnvalue_3 (Transformation|GetActorForwardVector _returnvalue))
  (bind _returnvalue_4 (* _returnvalue_3 7e+02))
  (bind _returnvalue_5 (+ _returnvalue_2 _returnvalue_4))
  (Variables|Default|SetRadius 6e+02)
  (bind (_outhits _returnvalue_6) (Collision|MultiSphereTraceForObjects _returnvalue_5 (+ _returnvalue_5 "1.000000, 0, 0") (Variables|Default|GetRadius) (Utilities|Array|MakeArray "ObjectTypeQuery7") false (Utilities|Array|MakeArray (Variables|Default|GetCurrentTarget)) "None" :!label _label))
  (if _returnvalue_6
    (Variables|Default|SetCurrentTarget (.HitActor (Collision|BreakHitResult (Utilities|Array|Get(acopy) _outhits (Math|Random|RandomInteger (Utilities|Array|Length _outhits))))))
    (CallFunction|Goto (.RandomLocation (AI|Navigation|GetRandomReachablePointinRadius (.ImpactPoint (Collision|BreakHitResult (Utilities|Array|Get(acopy) _outhits (Math|Random|RandomInteger (Utilities|Array|Length _outhits))))) 1e+02 0 0)))
    (else
      (Variables|Default|SetRadius (+ (Variables|Default|GetRadius) 5e+02))
      (Utilities|FlowControl|Delay 0.2)
      (goto _label))))